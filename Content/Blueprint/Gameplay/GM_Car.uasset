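; GM_Car is a game mode that manages a set of selectable cars, with one active at a time.
; On BeginPlay it takes row names from the game state's CarInfoList table, looks them up in DT_CarList, spawns and initializes each car actor, and activates the first.
; ChangeCar steps through the list without wrapping, calling Abandon and Use to swap cars.
; ChangeColour forwards a colour to the current car.
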(event EventBeginPlay
  (CallFunction|Init))

(event EventTick
  (params (DeltaSeconds :type Float%20%28single-precision%29)))

(fn ConstructionScript)

(fn Init
  (bind _carlist (Variables|Default|GetCarList))
  (bind _output (Utilities|Array|Get(acopy) _carlist))
  (bind _gamestate (Class|IBPGameState|CasttoGameState(Message) (Game|GetGameState)))
  (bind _output_get (Variables|Default|SetGame%20State _gamestate))
  (bind _outrownames (DataTable|GetDataTableRowNames (Variables|/Game/Blueprint/Gameplay/GS_Car.GS_Car_C|GetCarInfoList _output_get)))
  (for _array_element _outrownames
    (bind _returnvalue (Utilities|GetDataTableRow "/Game/Blueprint/Data/Datatable/DT_CarList.DT_CarList" _array_element)
      (:then
        (bind _returnvalue_2 (Game|SpawnActorfromClass (.CarActor (Utilities|Struct|BreakST_CarInfo _returnvalue)) (Math|Transform|MakeTransform "0, 0, 0" "0, 0, 0" "1.000000,1.000000,1.000000") "AlwaysSpawn" "MultiplyWithRoot" 0 0))
        (Default|Init _returnvalue_2 _returnvalue)
        (Utilities|Array|AddUnique (Variables|Default|GetCarList) _returnvalue_2))))
  (Default|Use _output)
  (Variables|Default|SetCurrCar _output)
  (Variables|Default|SetListLength (Utilities|Array|Length (Variables|Default|GetCarList))))

(fn ChangeCar
  (params (ChangeOption :type Enum_ChangeCar%20Enum :default "NewEnumerator0"))
  (switch Utilities|FlowControl|Switch|SwitchonEnum_ChangeCar ChangeOption
    (:NewEnumerator0
      (if (not (== (+ (Variables|Default|GetCar_Index) 1) (Variables|Default|GetListLength)))
        (bind _result (Math|Integer|IncrementInt (Variables|Default|GetCar_Index))
          (:%20%20
            (Utilities|IsValid (Utilities|Array|Get(acopy) (Variables|Default|GetCarList) _result)
              (:Is%20Valid
                (Default|Abandon (Variables|Default|GetCurrCar))
                (Default|Use (Utilities|Array|Get(acopy) (Variables|Default|GetCarList) _result))
                (Variables|Default|SetCurrCar (Utilities|Array|Get(acopy) (Variables|Default|GetCarList) _result))))))))
    (:NewEnumerator1
      (if (not (< (- (Variables|Default|GetCar_Index) 1) 0))
        (bind _result_2 (Math|Integer|DecrementInt (Variables|Default|GetCar_Index))
          (:%20%20
            (Utilities|IsValid (Utilities|Array|Get(acopy) (Variables|Default|GetCarList) _result_2)
              (:Is%20Valid
                (Default|Abandon (Variables|Default|GetCurrCar))
                (Default|Use (Utilities|Array|Get(acopy) (Variables|Default|GetCarList) _result_2))
                (Variables|Default|SetCurrCar (Utilities|Array|Get(acopy) (Variables|Default|GetCarList) _result_2))))))))))

(fn ChangeColour
  (params (Color :type Enum_ChangeColor%20Enum :default "NewEnumerator0"))
  (Default|ChangeColour (Variables|Default|GetCurrCar) Color))

(fn CasttoGameMode
  (return self))