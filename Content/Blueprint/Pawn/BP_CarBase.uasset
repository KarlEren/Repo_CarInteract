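; BP_CarBase is a car display pawn that shows a car mesh and spins it while the car is in use.
; Init takes a car info struct, applies its mesh and hides the actor.
; Use and Abandon toggle visibility and unpause or pause a looping timer created on BeginPlay.
; Each timer tick restarts a timeline that lerps the mesh's yaw in steps for continuous rotation.
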(event Custom|Rotate
  (bind _mesh_car (Variables|Default|GetMesh_Car))
  (bind _returnvalue (Transformation|GetWorldRotation _mesh_car))
  (bind (_roll _pitch _yaw) (Math|Rotator|BreakRotator _returnvalue))
  (bind _rotate (Timeline|Rotated PlayFromStart)
    (:Update
      (Transformation|SetWorldRotation (Variables|Default|GetMesh_Car) (Math|Rotator|Lerp(Rotator) _returnvalue (Math|Rotator|MakeRotator _roll _pitch (- _yaw 1e+01)) _rotate true) false false))))

(event EventBeginPlay
  (bind _returnvalue (Utilities|Time|SetTimerbyEvent (delegate Custom|Rotate) 0.1 true))
  (bind _output_get (Variables|Default|SetHandle_Rotate _returnvalue))
  (Utilities|Time|PauseTimerbyHandle _output_get))

(event Collision|EventActorBeginOverlap
  (params (OtherActor :type Actor%20Object%20Reference)))

(event EventTick
  (params (DeltaSeconds :type Float%20%28single-precision%29)))

(fn ConstructionScript)

(fn Init
  (params (CarInfo :type ST%20Car%20Info%20Structure))
  (bind _output_get (Variables|Default|SetCarInfo CarInfo))
  (bind _returnvalue (Components|StaticMesh|SetStaticMesh (Variables|Default|GetMesh_Car) (Utilities|Struct|BreakST_CarInfo _output_get)))
  (Rendering|SetActorHiddenInGame true)
  (return _returnvalue))

(fn Use
  (Variables|Default|SetInUse true)
  (Rendering|SetActorHiddenInGame false)
  (Utilities|Time|UnpauseTimerbyHandle (Variables|Default|GetHandle_Rotate)))

(fn Abandon
  (Variables|Default|SetInUse false)
  (Rendering|SetActorHiddenInGame true)
  (Utilities|Time|PauseTimerbyHandle (Variables|Default|GetHandle_Rotate)))