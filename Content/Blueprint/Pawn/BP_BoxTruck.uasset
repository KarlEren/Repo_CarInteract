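; Box truck pawn Blueprint, a child of a car parent class, that adds selectable exterior paint colours.
; ChangeColour switches on a colour option, creates a dynamic instance of the truck exterior material, sets its masked colour parameter and applies it to one material slot on MeshCar.
; Named options use fixed colours, while the default case takes the default colour from CarInfo.
; The event graph holds only disabled stubs, and construction defers to the parent.
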(event EventBeginPlay
  (|CallParentFunction) ; 此节点被禁用，将不会被调用。\n从引脚连出引线来编译功能。
)

(event Collision|EventActorBeginOverlap
  (params (OtherActor :type Actor%20Object%20Reference))
  (|CallParentFunction OtherActor) ; 此节点被禁用，将不会被调用。\n从引脚连出引线来编译功能。
)

(event EventTick
  (params (DeltaSeconds :type Float%20%28single-precision%29))
  (|CallParentFunction DeltaSeconds) ; 此节点被禁用，将不会被调用。\n从引脚连出引线来编译功能。
)

(fn ConstructionScript
  (|CallParentFunction))

(fn ChangeColour
  (params (ColourOption :type Enum_ChangeColor%20Enum :default "NewEnumerator0"))
  (switch Utilities|FlowControl|Switch|SwitchonEnum_ChangeColor ColourOption
    (:NewEnumerator0
      (bind _returnvalue (Rendering|Material|CreateDynamicMaterialInstance "/Game/Assets/VehicleVarietyVol2/Materials/BoxTruck/Mi_BoxTruck_Exterior_01a.Mi_BoxTruck_Exterior_01a" "None" "None" :!class /Script/Engine.KismetMaterialLibrary))
      (Rendering|Material|SetVectorParameterValue _returnvalue "03c - Masked Colour" (Utilities|Struct|BreakST_CarInfo (Variables|Default|GetCarInfo)) :!class /Script/Engine.MaterialInstanceDynamic)
      (Rendering|Material|SetMaterial (Variables|Default|GetMesh_Car) 4 _returnvalue))
    (:NewEnumerator1
      (bind _returnvalue_2 (Rendering|Material|CreateDynamicMaterialInstance "/Game/Assets/VehicleVarietyVol2/Materials/BoxTruck/Mi_BoxTruck_Exterior_01a.Mi_BoxTruck_Exterior_01a" "None" "None" :!class /Script/Engine.KismetMaterialLibrary))
      (Rendering|Material|SetVectorParameterValue _returnvalue_2 "03c - Masked Colour" (Utilities|Struct|MakeLinearColor 0.0 0.0 1.0 0.0) :!class /Script/Engine.MaterialInstanceDynamic)
      (Rendering|Material|SetMaterial (Variables|Default|GetMesh_Car) 4 _returnvalue_2))
    (:NewEnumerator2
      (bind _returnvalue_3 (Rendering|Material|CreateDynamicMaterialInstance "/Game/Assets/VehicleVarietyVol2/Materials/BoxTruck/Mi_BoxTruck_Exterior_01a.Mi_BoxTruck_Exterior_01a" "None" "None" :!class /Script/Engine.KismetMaterialLibrary))
      (Rendering|Material|SetVectorParameterValue _returnvalue_3 "03c - Masked Colour" (Utilities|Struct|MakeLinearColor 1.0 0.0 0.0 0.0) :!class /Script/Engine.MaterialInstanceDynamic)
      (Rendering|Material|SetMaterial (Variables|Default|GetMesh_Car) 4 _returnvalue_3))
    (:NewEnumerator3
      (bind _returnvalue_4 (Rendering|Material|CreateDynamicMaterialInstance "/Game/Assets/VehicleVarietyVol2/Materials/BoxTruck/Mi_BoxTruck_Exterior_01a.Mi_BoxTruck_Exterior_01a" "None" "None" :!class /Script/Engine.KismetMaterialLibrary))
      (Rendering|Material|SetVectorParameterValue _returnvalue_4 "03c - Masked Colour" (Utilities|Struct|MakeLinearColor 0.0 0.0 0.0 0.0) :!class /Script/Engine.MaterialInstanceDynamic)
      (Rendering|Material|SetMaterial (Variables|Default|GetMesh_Car) 4 _returnvalue_4))
    (:NewEnumerator4
      (bind _returnvalue_5 (Rendering|Material|CreateDynamicMaterialInstance "/Game/Assets/VehicleVarietyVol2/Materials/BoxTruck/Mi_BoxTruck_Exterior_01a.Mi_BoxTruck_Exterior_01a" "None" "None" :!class /Script/Engine.KismetMaterialLibrary))
      (Rendering|Material|SetVectorParameterValue _returnvalue_5 "03c - Masked Colour" (Utilities|Struct|MakeLinearColor 1.0 1.0 1.0 1.0) :!class /Script/Engine.MaterialInstanceDynamic)
      (Rendering|Material|SetMaterial (Variables|Default|GetMesh_Car) 4 _returnvalue_5))))